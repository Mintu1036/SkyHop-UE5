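; Finish line trigger actor that ends the level when the player character overlaps its box.
; The overlap disables input, shows LevelFinish_UI with a mouse cursor and UI-only input, and removes the MainHUB_UI HUD.
; It then parses the number from the current level name, uses it as the index to set in the game instance save's LevelUnlock array, and saves to disk.
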(event `self.Box.OnComponentBeginOverlap`
  (params (OverlappedComponent :type "PrimitiveComponent Object Reference") (OtherActor :type "Actor Object Reference") (OtherComp :type "PrimitiveComponent Object Reference") (OtherBodyIndex :type Integer) (bFromSweep :type Boolean) (SweepResult :type "HitResult Structure (by ref)"))
  (bind _returnvalue (`GameplayStatics.GetPlayerController` 0))
  (if (== OtherActor (`GameplayStatics.GetPlayerCharacter` 0))
    (`self.DisableInput` (`GameplayStatics.GetPlayerController` 0))
    (bind _returnvalue_2 (`|CreateWidget` "/Game/UserWidget/LevelFinish_UI.LevelFinish_UI_C"))
    (`UserWidget.AddToViewport` _returnvalue_2 0)
    (`WidgetBlueprintLibrary.SetInputMode_UIOnlyEx` _returnvalue null)
    (set `PlayerController.bShowMouseCursor` true _returnvalue)
    (bind _foundwidgets (`WidgetBlueprintLibrary.GetAllWidgetsOfClass` "/Game/UserWidget/MainHUB_UI.MainHUB_UI_C"))
    (`Widget.RemoveFromParent` (`|GetArrayItem` _foundwidgets))
    (`self.Unlock New Level`)))

(event `Unlock New Level`
  (bind _asmy_game_instance_bp (cast `/Game/Blueprints/MyGameInstance_BP` (`GameplayStatics.GetGameInstance`)))
  (bind _returnvalue (`GameplayStatics.GetCurrentLevelName` true))
  (bind _save_game_ref (`/Game/Blueprints/MyGameInstance_BP.Save Game Ref` _asmy_game_instance_bp))
  (`KismetArrayLibrary.Array_Set` (`/Game/Blueprints/MySaveGame_BP.Level Unlock` _save_game_ref) (`KismetStringLibrary.Conv_StringToInt` (`KismetStringLibrary.GetSubstring` _returnvalue 5 10)) true)
  (`GameplayStatics.SaveGameToSlot` _save_game_ref "Slot1"))

(fn `UserConstructionScript`)