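; Kill zone actor that ends the game when the player character enters its trigger box.
; On overlap with the player, it destroys the character and shows a "Game Over" widget.
; It then switches the player controller to UI-only input with a visible cursor and removes the main HUB UI held by MyGameMode.
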(event `self.KillZ Box.OnComponentBeginOverlap`
  (params (OverlappedComponent :type "PrimitiveComponent Object Reference") (OtherActor :type "Actor Object Reference") (OtherComp :type "PrimitiveComponent Object Reference") (OtherBodyIndex :type Integer) (bFromSweep :type Boolean) (SweepResult :type "HitResult Structure (by ref)"))
  (bind _returnvalue (`GameplayStatics.GetPlayerCharacter` 0))
  (bind _returnvalue_2 (`GameplayStatics.GetPlayerController` 0))
  (if (== OtherActor _returnvalue)
    (`self.K2_DestroyActor` _returnvalue)
    (bind _returnvalue_3 (`|CreateWidget` "/Game/UserWidget/GameOverUI.GameOverUI_C" null "Game Over"))
    (`UserWidget.AddToViewport` _returnvalue_3 0)
    (`WidgetBlueprintLibrary.SetInputMode_UIOnlyEx` _returnvalue_2 null)
    (set `PlayerController.bShowMouseCursor` true _returnvalue_2)
    (bind _asmy_game_mode (cast `/Game/Blueprints/MyGameMode` (`GameplayStatics.GetGameMode`)))
    (`Widget.RemoveFromParent` (`/Game/Blueprints/MyGameMode.MainHUB_UI` _asmy_game_mode))))

(fn `UserConstructionScript`)