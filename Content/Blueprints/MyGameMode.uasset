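; Game mode Blueprint that sets up the player's main HUD and tracks the currency total.
; On BeginPlay it switches to game-only input, hides the cursor, adds the MainHUB_UI widget to the viewport and caches the game instance.
; UpdateCurrency adds an amount to the value parsed from the HUD text and separately to the save game's CurrencyAmount, then writes the save to its slot immediately.
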(event `self.ReceiveBeginPlay`
  (bind _returnvalue (`GameplayStatics.GetPlayerController` 0))
  (`WidgetBlueprintLibrary.SetInputMode_GameOnly` _returnvalue)
  (set `PlayerController.bShowMouseCursor` false _returnvalue)
  (bind _returnvalue_2 (`|CreateWidget` "/Game/UserWidget/MainHUB_UI.MainHUB_UI_C"))
  (bind _output_get (set `self.MainHUB_UI` _returnvalue_2))
  (`UserWidget.AddToViewport` _output_get 0)
  (bind _asmy_game_instance_bp (cast `/Game/Blueprints/MyGameInstance_BP` (`GameplayStatics.GetGameInstance`)))
  (set `self.Game Instance Ref` _asmy_game_instance_bp))

(event `Update Currency`
  (params (`Add Amount` :type Integer))
  (bind _save_game_ref (`/Game/Blueprints/MyGameInstance_BP.Save Game Ref` (`self.Game Instance Ref`)))
  (`TextBlock.SetText` (`/Game/UserWidget/MainHUB_UI.Currency_Amt` (`self.MainHUB_UI`)) (`KismetTextLibrary.Conv_IntToText` (+ `Add Amount` (`KismetStringLibrary.Conv_StringToInt` (`KismetTextLibrary.Conv_TextToString` (`TextBlock.GetText` (`/Game/UserWidget/MainHUB_UI.Currency_Amt` (`self.MainHUB_UI`))))))))
  (set `/Game/Blueprints/MySaveGame_BP.Currency Amount` (+ `Add Amount` (`/Game/Blueprints/MySaveGame_BP.Currency Amount` _save_game_ref)) _save_game_ref)
  (`GameplayStatics.SaveGameToSlot` _save_game_ref "Slot1"))

(fn `UserConstructionScript`)