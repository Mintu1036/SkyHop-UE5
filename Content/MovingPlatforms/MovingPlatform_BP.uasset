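; MovingPlatform_BP is a platform that moves back and forth endlessly between its starting position and an end location.
; On BeginPlay it stores the mesh's relative location and starts a fast looping timer, used in place of Tick.
; Each timer call advances an alpha by Speed, lerps the mesh's relative location without sweep, and reverses Speed at either end of the path.
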(event `self.ReceiveBeginPlay`
  (`self.Move Platform`))

(event `Move Platform`
  (set `self.Start Loc` (`SceneComponent.RelativeLocation` (`self.StaticMesh`)))
  (`KismetSystemLibrary.K2_SetTimerDelegate` (delegate `Start Moving`) 0.005 true))

(event `Start Moving`
  (bind _alpha (`self.Alpha`))
  (set `self.Alpha` (+ (`self.Alpha`) (`self.Speed`)))
  (`SceneComponent.K2_SetRelativeLocation` (`self.StaticMesh`) (`KismetMathLibrary.VLerp` (`self.Start Loc`) (`self.End Loc`) _alpha) false false)
  (`|ExecutionSequence`
    (:`then_0`
      (if (>= _alpha 1.0)
        (set `self.Speed` -0.002)))
    (:`then_1`
      (if (<= _alpha 0.0)
        (set `self.Speed` 0.002)))))

(fn `UserConstructionScript`)