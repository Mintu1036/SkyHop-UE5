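; Rotating obstacle that spins at a configurable speed and knocks the player character away on contact.
; On BeginPlay, Speed sets a single axis of the RotatingMovement component's rotation rate.
; When InteractiveBox2 overlaps the player, it launches them using a MakeRotFromZ result built from the mesh's physics angular velocity multiplied by the impact point, then scaled up.
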(event `self.ReceiveBeginPlay`
  (set `RotatingMovementComponent.RotationRate` (`KismetMathLibrary.MakeRotator` 0.0 (`self.Speed`)) (`self.RotatingMovement`)))

(event `self.Interactive Box2.OnComponentBeginOverlap`
  (params (OverlappedComponent :type "PrimitiveComponent Object Reference") (OtherActor :type "Actor Object Reference") (OtherComp :type "PrimitiveComponent Object Reference") (OtherBodyIndex :type Integer) (bFromSweep :type Boolean) (SweepResult :type "HitResult Structure (by ref)"))
  (bind _returnvalue (`GameplayStatics.GetPlayerCharacter` 0))
  (if (== null _returnvalue)
    (`Character.LaunchCharacter` _returnvalue (* (`KismetMathLibrary.MakeRotFromZ` (* (`PrimitiveComponent.GetPhysicsAngularVelocityInDegrees` (`self.Obstacle Mesh`) "None") (`.ImpactPoint` (`GameplayStatics.BreakHitResult` SweepResult)))) 1000.0) false false)))

(fn `UserConstructionScript`
  (`parent.UserConstructionScript`))